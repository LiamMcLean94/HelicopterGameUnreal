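; Player-controlled physics helicopter that flies through a thruster and input-driven torques, with a mouse-orbited spring arm camera.
; On BeginPlay it shifts the mesh's center of mass in X and Y to line up with the thruster.
; Move Up varies thrust around a mass-scaled, near-hover baseline.
; Rotate Right applies yaw torque, while tilt inputs combine with current pitch or roll, clamped, to produce self-leveling, mass-independent torque.
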(event Collision|EventActorBeginOverlap
  (params (OtherActor :type Actor%20Object%20Reference)))

(event EventTick
  (params (DeltaSeconds :type Float%20%28single-precision%29)))

(event EventBeginPlay
  (bind _physicsthruster (Variables|Default|GetPhysicsThruster))
  (bind _staticmesh (Variables|Default|GetStaticMesh))
  (bind _staticmesh_2 (Variables|Default|GetStaticMesh))
  (bind _returnvalue (Transformation|GetWorldLocation _physicsthruster))
  (bind _returnvalue_2 (Physics|GetCenterOfMass _staticmesh "None"))
  (bind _returnvalue_3 (Transformation|GetWorldRotation _staticmesh_2))
  (bind _returnvalue_4 (Class|KismetMathLibrary|NegateRotator _returnvalue_3))
  (bind _returnvalue_5 (- _returnvalue _returnvalue_2))
  (bind _returnvalue_6 (Math|Vector|RotateVector _returnvalue_5 _returnvalue_4))
  (Class|PrimitiveComponent|SetCenterOfMass (Variables|Default|GetStaticMesh) (Math|Vector|MakeVector (.x _returnvalue_6) (.y _returnvalue_6) 0.0) "None"))

(event Input|AxisEvents|InputAxisMouseRight
  (params (AxisValue :type Float%20%28single-precision%29))
  ;[1 1 1] Camera Look Around
  (Transformation|AddRelativeRotation (Variables|Default|GetSpringArm) (Math|Rotator|MakeRotator 0.0 0.0 AxisValue) false false))

(event Input|AxisEvents|InputAxisMouseUp
  (params (AxisValue :type Float%20%28single-precision%29))
  ;[1 1 1] Camera Look Around
  (Transformation|AddRelativeRotation (Variables|Default|GetSpringArm) (Math|Rotator|MakeRotator 0.0 AxisValue 0.0) false false))

(event Input|AxisEvents|InputAxisMoveUp
  (params (AxisValue :type Float%20%28single-precision%29))
  ;[1 1 1] Move up/Down
  (Variables|/Script/Engine.PhysicsThrusterComponent|SetThrustStrength (Variables|Default|GetPhysicsThruster) (* (+ (* AxisValue 2e+02) 9.7e+02) (Physics|GetMass (Variables|Default|GetStaticMesh)))))

(event Input|AxisEvents|InputAxisRotateRight
  (params (AxisValue :type Float%20%28single-precision%29))
  (Class|PrimitiveComponent|AddTorqueinDegrees (Variables|Default|GetStaticMesh) (* AxisValue (Transformation|GetActorUpVector) 6e+01) "None" true))

(event Input|AxisEvents|InputAxisTiltForward
  (params (AxisValue :type Float%20%28single-precision%29))
  (Class|PrimitiveComponent|AddTorqueinDegrees (Variables|Default|GetStaticMesh) (* (Transformation|GetActorRightVector) (Math|Float|Clamp(Float) (+ (* AxisValue 3e+01) (.pitch (Transformation|GetWorldRotation (Variables|Default|GetStaticMesh)))) -2e+01 2e+01) 5.0) "None" true))

(event Input|AxisEvents|InputAxisTiltRight
  (params (AxisValue :type Float%20%28single-precision%29))
  (Class|PrimitiveComponent|AddTorqueinDegrees (Variables|Default|GetStaticMesh) (* (Transformation|GetActorForwardVector) (Math|Float|Clamp(Float) (+ (* AxisValue -3e+01) (.roll (Transformation|GetWorldRotation (Variables|Default|GetStaticMesh)))) -2e+01 2e+01) 5.0) "None" true))

(fn ConstructionScript)