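; BP_Helicopter is a player-controlled Huey helicopter with mouse camera look and vertical flight.
; Mouse axes add relative yaw and pitch rotation to the SpringArm to orbit the camera.
; The Move Up axis drives a PhysicsThruster, scaling thrust by the mesh's mass around a baseline just under default gravity, so input raises or lowers the craft independent of weight.
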(event Input|AxisEvents|InputAxisMouseRight
  (params (AxisValue :type Float%20%28single-precision%29))
  ;[1 1 1] Camera Look Around
  (Transformation|AddRelativeRotation (Variables|Default|GetSpringArm) (Math|Rotator|MakeRotator 0.0 0.0 AxisValue) false false))

(event Input|AxisEvents|InputAxisMouseUp
  (params (AxisValue :type Float%20%28single-precision%29))
  ;[1 1 1] Camera Look Around
  (Transformation|AddRelativeRotation (Variables|Default|GetSpringArm) (Math|Rotator|MakeRotator 0.0 AxisValue 0.0) false false))

(event Input|AxisEvents|InputAxisMoveUp
  (params (AxisValue :type Float%20%28single-precision%29))
  ;[1 1 1] Move up/Down
  (Variables|/Script/Engine.PhysicsThrusterComponent|SetThrustStrength (Variables|Default|GetPhysics%20Thruster) (* (+ (* AxisValue 1e+02) 9.7e+02) (Physics|GetMass (Variables|Default|GetSK_HB_HUEY)))))

(fn ConstructionScript)